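; Interactable bench task actor that plays a short sit-on-bench camera sequence for the TopDownCharacter.
; Trigger overlap enables input and opens a Gate, letting the interact press start a DoOnce-guarded sequence.
; It blends to the bench camera, hides and freezes the character, and pans right, left, then right via counted Delay loops.
; It then returns the view and control, shows the character and sets SatAtBench.
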(event `Right`
  (bind _right_count (`self.Right Count`))
  ;[1 1 1] Camera Rotate Right Movement
  (if (not (== _right_count 0)) :!label _label
    (`SceneComponent.K2_AddWorldRotation` (`self.Front`) (struct :`Yaw` -2.0) false false)
    (set `self.Right Count` (- _right_count 1))
    (`KismetSystemLibrary.Delay` 0.01)
    (goto _label)))

(event `Left`
  (bind _left_count (`self.Left Count`))
  ;[1 1 1] Camera Rotate Left Movement
  (if (not (== _left_count 0)) :!label _label_2
    (`SceneComponent.K2_AddWorldRotation` (`self.Front`) (struct :`Yaw` 2.0) false false)
    (set `self.Left Count` (- _left_count 1))
    (`KismetSystemLibrary.Delay` 0.01)
    (goto _label_2)))

(event `self.ReceiveBeginPlay`
  (`self.DisableInput` (`GameplayStatics.GetPlayerController` 0)))

(event `InputAction|Intereact`
  (params (Key :type "Key Structure"))
  (bind _as_top_down_character (`self.As Top Down Character`))
  (bind _as_top_down_character_2 (`self.As Top Down Character`))
  (:`Pressed`
    (`/Engine/EditorBlueprintResources/StandardMacros.Gate` true :!label _label_3
      (:`Exit`
        (`/Engine/EditorBlueprintResources/StandardMacros.DoOnce` false :!label _label_4
          (:`Completed`
            ;[1 1 1] Move to bench Camera and hidden player
            (`PlayerController.SetViewTargetWithBlend` (`GameplayStatics.GetPlayerController` 0) (`ActorComponent.GetOwner` (`self.Front`)) 1.0 "VTBlend_Linear" 0.0 false)
            (`KismetSystemLibrary.Delay` 0.85)
            (`SceneComponent.SetHiddenInGame` (`Character.Mesh` _as_top_down_character) true false)
            (`SceneComponent.SetHiddenInGame` (`/Game/Character/TopDownCharacter.CH` _as_top_down_character) true false)
            (`self.DisableInput` _as_top_down_character (`GameplayStatics.GetPlayerController` 0))
            ;[1 1 1] Movement Order
            (`KismetSystemLibrary.Delay` 2.0)
            (`self.Right`)
            (`KismetSystemLibrary.Delay` 3.2)
            (`self.Left`)
            (`KismetSystemLibrary.Delay` 2.5)
            (set `self.Right Count` 25)
            (`self.Right`)
            (`KismetSystemLibrary.Delay` 1.0)
            ;[1 1 1] Move to PLayer Camera And Show PLayer
            (`PlayerController.SetViewTargetWithBlend` (`GameplayStatics.GetPlayerController` 0) (`GameplayStatics.GetPlayerCharacter` 0) 1.0 "VTBlend_Linear" 0.0 false)
            (`KismetSystemLibrary.Delay` 0.5)
            (`SceneComponent.SetHiddenInGame` (`Character.Mesh` _as_top_down_character_2) false false)
            (`self.EnableInput` _as_top_down_character_2 (`GameplayStatics.GetPlayerController` 0))
            ;[1 1 1] set task done in player
            (set `/Game/Character/TopDownCharacter.sat at bench` true (`self.As Top Down Character`))
            (goto _label_4 :!via `Reset`)))))))

(event `self.Trigger.OnComponentBeginOverlap`
  (params (OverlappedComponent :type "PrimitiveComponent Object Reference") (OtherActor :type "Actor Object Reference") (OtherComp :type "PrimitiveComponent Object Reference") (OtherBodyIndex :type Integer) (bFromSweep :type Boolean) (SweepResult :type "HitResult Structure (by ref)"))
  ;[1 1 1] Overlapp Events
  (bind _astop_down_character (cast `/Game/Character/TopDownCharacter` OtherActor))
  (set `self.As Top Down Character` _astop_down_character)
  (`self.EnableInput` (`GameplayStatics.GetPlayerController` 0))
  (goto _label_3 :!via `Open`))

(event `self.Trigger.OnComponentEndOverlap`
  (params (OverlappedComponent :type "PrimitiveComponent Object Reference") (OtherActor :type "Actor Object Reference") (OtherComp :type "PrimitiveComponent Object Reference") (OtherBodyIndex :type Integer))
  ;[1 1 1] Overlapp Events
  (cast `/Game/Character/TopDownCharacter` OtherActor)
  (goto _label_3 :!via `Close`))

(fn `UserConstructionScript`)