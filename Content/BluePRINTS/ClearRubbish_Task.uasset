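; Rubbish pile task actor that the player clears by holding the Intereact input while inside its sphere.
; Overlap opens a gate for the input, which zooms the camera in stepped delays, shows dust and a camera-facing progress widget.
; A delayed loop raises progress while held; on completion it decrements the player's TrashAmount and destroys itself.
; BeginPlay seeds that TrashAmount from AmountOfTrash, and the construction script applies the chosen mesh.
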(event `self.ReceiveBeginPlay`
  (`self.DisableInput` (`GameplayStatics.GetPlayerController` 0))
  ;[1 1 1] Cast to player and set rubbish variable for player
  (bind _astop_down_character (cast `/Game/Character/TopDownCharacter` (`GameplayStatics.GetPlayerCharacter` 0)))
  (bind _output_get (set `self.As Top Down Character` _astop_down_character))
  (set `/Game/Character/TopDownCharacter.Trash Amount` (`self.Amount of Trash`) _output_get))

(event `self.ReceiveTick`
  (params (DeltaSeconds :type "Float (single-precision)"))
  ;[1 1 1] Set look at rotation for Progress Bar
  (`SceneComponent.K2_SetWorldRotation` (`self.Widget`) (`KismetMathLibrary.FindLookAtRotation` (`SceneComponent.K2_GetComponentLocation` (`self.Widget`)) (`SceneComponent.K2_GetComponentLocation` (`/Game/Character/TopDownCharacter.Camera1` (`self.As Top Down Character`)))) false false))

(event `InputAction|Intereact`
  (params (Key :type "Key Structure"))
  (bind _current_task_progress_bar (`self.current Task Progress Bar`))
  (:`Pressed`
    (set `self.Pressed` true)
    (`/Engine/EditorBlueprintResources/StandardMacros.Gate` true :!label _label
      (:`Exit`
        (`|ExecutionSequence`
          (:`then_0`
            (`self.Zoom in`)
            (`SceneComponent.SetHiddenInGame` (`self.Dust`) false false)
            ;[1 1 1] Toggle visibilty when near
            (`SceneComponent.SetVisibility` (`self.Widget`) true false)
            ;[1 1 1] Check If Task is done
            (if (>= (`self.current Task Progress Bar`) 1.0)
              (`self.Zoom out`)
              ;[1 1 1] Remove 1 Rubbish from player
              (bind _astop_down_character (cast `/Game/Character/TopDownCharacter` (`GameplayStatics.GetPlayerCharacter` 0) :!label _label_2))
              (set `/Game/Character/TopDownCharacter.Trash Amount` (- (`/Game/Character/TopDownCharacter.Trash Amount` _astop_down_character) 1) _astop_down_character)
              (`ActorComponent.K2_DestroyComponent` (`self.StaticMesh`))
              (`ActorComponent.K2_DestroyComponent` (`self.Dust`))
              (`KismetSystemLibrary.Delay` 0.4)
              (`self.K2_DestroyActor`)))
          (:`then_1`
            ;[1 1 1] Check If Key Is Pressed
            (if (`self.Pressed`) :!label _label_3
              ;[1 1 1] Check if task is done
              (if (>= (`self.current Task Progress Bar`) 1.0)
                (goto _label_2)
                (else
                  ;[1 1 1] Progress Bar Lerp
                  (set `self.current Task Progress Bar` (`KismetMathLibrary.Lerp` _current_task_progress_bar (+ (`self.Amount Of Progress to add to task `) _current_task_progress_bar) 0.4))
                  (`KismetSystemLibrary.Delay` (`self.Time Delay between each progression`))
                  (goto _label_3)))))))))
  (:`Released`
    (set `self.Pressed` false)))

(event `self.Sphere.OnComponentBeginOverlap`
  (params (OverlappedComponent :type "PrimitiveComponent Object Reference") (OtherActor :type "Actor Object Reference") (OtherComp :type "PrimitiveComponent Object Reference") (OtherBodyIndex :type Integer) (bFromSweep :type Boolean) (SweepResult :type "HitResult Structure (by ref)"))
  (bind _astop_down_character (cast `/Game/Character/TopDownCharacter` OtherActor))
  ;[1 1 1] Overlapp Events
  (set `self.As Top Down Character_0` _astop_down_character)
  (`self.EnableInput` (`GameplayStatics.GetPlayerController` 0))
  (goto _label :!via `Open`))

(event `self.Sphere.OnComponentEndOverlap`
  (params (OverlappedComponent :type "PrimitiveComponent Object Reference") (OtherActor :type "Actor Object Reference") (OtherComp :type "PrimitiveComponent Object Reference") (OtherBodyIndex :type Integer))
  ;[1 1 1] Overlapp Events
  (cast `/Game/Character/TopDownCharacter` OtherActor)
  (`self.Zoom out`)
  ;[1 1 1] Toggle visibilty when near
  (`SceneComponent.SetVisibility` (`self.Widget`) false false)
  (`SceneComponent.SetVisibility` (`self.Dust`) false false)
  (goto _label :!via `Close`))

(event `Zoom in`
  (bind _springarm1 (`/Game/Character/TopDownCharacter.SpringArm1` (`self.As Top Down Character_0`)))
  ;[1 1 1] Zoom IN And OUt Events
  (set `SpringArmComponent.TargetArmLength` 760.0 _springarm1)
  (`KismetSystemLibrary.Delay` 0.1)
  (set `SpringArmComponent.TargetArmLength` 720.0 _springarm1)
  (`KismetSystemLibrary.Delay` 0.1)
  (set `SpringArmComponent.TargetArmLength` 680.0 _springarm1)
  (`KismetSystemLibrary.Delay` 0.1)
  (set `SpringArmComponent.TargetArmLength` 640.0 _springarm1)
  (`KismetSystemLibrary.Delay` 0.1)
  (set `SpringArmComponent.TargetArmLength` 600.0 _springarm1)
  (`KismetSystemLibrary.Delay` 0.1))

(event `Zoom out`
  (bind _springarm1 (`/Game/Character/TopDownCharacter.SpringArm1` (`self.As Top Down Character_0`)))
  ;[1 1 1] Zoom IN And OUt Events
  (set `SpringArmComponent.TargetArmLength` 640.0 _springarm1)
  (`KismetSystemLibrary.Delay` 0.1)
  (set `SpringArmComponent.TargetArmLength` 680.0 _springarm1)
  (`KismetSystemLibrary.Delay` 0.1)
  (set `SpringArmComponent.TargetArmLength` 720.0 _springarm1)
  (`KismetSystemLibrary.Delay` 0.1)
  (set `SpringArmComponent.TargetArmLength` 760.0 _springarm1)
  (`KismetSystemLibrary.Delay` 0.1)
  (set `SpringArmComponent.TargetArmLength` 800.0 _springarm1)
  (`KismetSystemLibrary.Delay` 0.1))

(fn `UserConstructionScript`
  (set `self.StaticMesh` (`self.Mesh`)))