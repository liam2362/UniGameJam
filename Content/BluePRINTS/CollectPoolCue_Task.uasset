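; Pool cue pickup actor that the TopDownCharacter collects with the interact input.
; The sphere's overlap events cache the character and open or close a gate, so the input only works while the character is in range.
; Collecting sets PoolCueCollected on the character and briefly shows the Stars particles before hiding them with the cue and destroying the actor.
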(event `InputAction|Intereact`
  (params (Key :type "Key Structure"))
  (:`Pressed`
    (`/Engine/EditorBlueprintResources/StandardMacros.Gate` true :!label _label
      (:`Exit`
        (set `/Game/Character/TopDownCharacter.Pool Cue Collected` true (`self.As Top Down Character_0`))
        ;[1 1 1] Show Particles
        (`SceneComponent.SetHiddenInGame` (`self.Stars`) false false)
        (`KismetSystemLibrary.Delay` 0.6)
        (`SceneComponent.SetHiddenInGame` (`self.Stars`) true false)
        (`SceneComponent.SetHiddenInGame` (`self.CUe`) true false)
        (`self.K2_DestroyActor`)))))

(event `self.Sphere.OnComponentBeginOverlap`
  (params (OverlappedComponent :type "PrimitiveComponent Object Reference") (OtherActor :type "Actor Object Reference") (OtherComp :type "PrimitiveComponent Object Reference") (OtherBodyIndex :type Integer) (bFromSweep :type Boolean) (SweepResult :type "HitResult Structure (by ref)"))
  ;[1 1 1] Overlapp Events
  (bind _astop_down_character (cast `/Game/Character/TopDownCharacter` OtherActor))
  (set `self.As Top Down Character_0` _astop_down_character)
  (goto _label :!via `Open`))

(event `self.Sphere.OnComponentEndOverlap`
  (params (OverlappedComponent :type "PrimitiveComponent Object Reference") (OtherActor :type "Actor Object Reference") (OtherComp :type "PrimitiveComponent Object Reference") (OtherBodyIndex :type Integer))
  ;[1 1 1] Overlapp Events
  (cast `/Game/Character/TopDownCharacter` OtherActor)
  (goto _label :!via `Close`))

(fn `UserConstructionScript`
  (set `self.Cue Mesh` (`self.CUe`)))