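; A collectible solid-ball task actor that the TopDownCharacter picks up by pressing the interact input while in range.
; Sphere overlap opens and closes a gate on that input and stores the character reference.
; Interacting sets SoildBallsCollected from StripedBallsCollected plus one, flagging AllSoildBallsCollected when it equals the required total.
; It then briefly shows Stars particles before hiding them and the ball and destroying itself.
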(event `InputAction|Intereact`
  (params (Key :type "Key Structure"))
  (bind _as_top_down_character_0 (`self.As Top Down Character_0`))
  (:`Pressed`
    (`/Engine/EditorBlueprintResources/StandardMacros.Gate` true :!label _label
      (:`Exit`
        ;[1 1 1] Add 1 To the amount collected and check if the player has all of them
        (bind _output_get (set `/Game/Character/TopDownCharacter.Soild Balls Collected` (+ (`/Game/Character/TopDownCharacter.Striped Balls Collected` _as_top_down_character_0) 1) _as_top_down_character_0))
        (if (== _output_get (`self.How many Soild Balls Are Need`))
          (set `/Game/Character/TopDownCharacter.All Soild Balls Collected` true (`self.As Top Down Character_0`)))
        ;[1 1 1] Show Particles
        (`SceneComponent.SetHiddenInGame` (`self.Stars`) false false)
        (`KismetSystemLibrary.Delay` 0.6)
        (`SceneComponent.SetHiddenInGame` (`self.Stars`) true false)
        (`SceneComponent.SetHiddenInGame` (`self.Ball`) true false)
        (`self.K2_DestroyActor`)))))

(event `self.Sphere.OnComponentBeginOverlap`
  (params (OverlappedComponent :type "PrimitiveComponent Object Reference") (OtherActor :type "Actor Object Reference") (OtherComp :type "PrimitiveComponent Object Reference") (OtherBodyIndex :type Integer) (bFromSweep :type Boolean) (SweepResult :type "HitResult Structure (by ref)"))
  ;[1 1 1] Overlapp Events
  (bind _astop_down_character (cast `/Game/Character/TopDownCharacter` OtherActor))
  (set `self.As Top Down Character_0` _astop_down_character)
  (goto _label :!via `Open`))

(event `self.Sphere.OnComponentEndOverlap`
  (params (OverlappedComponent :type "PrimitiveComponent Object Reference") (OtherActor :type "Actor Object Reference") (OtherComp :type "PrimitiveComponent Object Reference") (OtherBodyIndex :type Integer))
  ;[1 1 1] Overlapp Events
  (cast `/Game/Character/TopDownCharacter` OtherActor)
  (goto _label :!via `Close`))

(fn `UserConstructionScript`
  (set `self.Cue Mesh` (`self.Ball`)))